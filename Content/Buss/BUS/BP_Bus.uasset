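; Drivable bus actor with a forward, neutral and reverse drive mode, set by overlapping button components or calling mode events.
; Tick moves the bus by local offsets: accelerating to a speed cap, reversing up to half that, or easing to a stop in neutral.
; Steering events rotate the wheel component and, above a minimum speed, yaw the actor proportionally to signed speed.
; ApplyUpgrade is an empty stub.
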(event `self.ReceiveTick`
  (params (DeltaSeconds :type "Float (single-precision)"))
  (switch `int` (`self.DriveMode`)
    (:`-1`
      (`self.DriveDown`))
    (:`0`
      (`self.DriveNeutral`))
    (:`1`
      (`self.DriveUp`))))

(event `self.ReceiveBeginPlay`)

(event `TurnWheelRight`
  (`SceneComponent.K2_AddLocalRotation` (`self.Steering_Wheel`) (struct :`Roll` 15.0) false false)
  (if (> (`KismetMathLibrary.Abs` (`self.Speed`)) 10.0)
    (`self.DriveRight`)))

(event `self.Btn_DriveUp.OnComponentBeginOverlap`
  (params (OverlappedComponent :type "PrimitiveComponent Object Reference") (OtherActor :type "Actor Object Reference") (OtherComp :type "PrimitiveComponent Object Reference") (OtherBodyIndex :type Integer) (bFromSweep :type Boolean) (SweepResult :type "HitResult Structure (by ref)"))
  (`self.SetModeForWard`)
  (set `self.DriveMode` 1 :!label _label)
  (`KismetSystemLibrary.PrintString` "Btn_DriveUp activado (DriveMode = 1)"))

(event `SetModeForWard`
  (goto _label))

(event `TurnWheelLeft`
  (`SceneComponent.K2_AddLocalRotation` (`self.Steering_Wheel`) (struct :`Roll` -15.0) false false)
  (if (> (`KismetMathLibrary.Abs` (`self.Speed`)) 10.0)
    (`self.DriveLeft`)))

(event `self.Btn_DriveNeutral.OnComponentBeginOverlap`
  (params (OverlappedComponent :type "PrimitiveComponent Object Reference") (OtherActor :type "Actor Object Reference") (OtherComp :type "PrimitiveComponent Object Reference") (OtherBodyIndex :type Integer) (bFromSweep :type Boolean) (SweepResult :type "HitResult Structure (by ref)"))
  (`self.SetModeNeutral`)
  (set `self.DriveMode` 0 :!label _label_2))

(event `SetModeNeutral`
  (goto _label_2))

(event `self.Btn_DriveDown.OnComponentBeginOverlap`
  (params (OverlappedComponent :type "PrimitiveComponent Object Reference") (OtherActor :type "Actor Object Reference") (OtherComp :type "PrimitiveComponent Object Reference") (OtherBodyIndex :type Integer) (bFromSweep :type Boolean) (SweepResult :type "HitResult Structure (by ref)"))
  (`self.SetModeReserve`)
  (set `self.DriveMode` -1 :!label _label_3))

(event `SetModeReserve`
  (goto _label_3))

(fn `ApplyUpgrade`
  (params (Upgrade :type "PDA_Upgrade Object Reference"))
  (locals (NewLocalVar :type "PDA_Upgrade Object Reference")))

(fn `DriveDown`
  (bind _output_get (set `self.Speed` (`KismetMathLibrary.FClamp` (- (`self.Speed`) (* 500.0 (`GameplayStatics.GetWorldDeltaSeconds`))) (* (`self.SpeedMAx`) -0.5))))
  (`self.K2_AddActorLocalOffset` (`KismetMathLibrary.MakeVector` (* _output_get (`GameplayStatics.GetWorldDeltaSeconds`)))))

(fn `DriveLeft`
  (if (> (`KismetMathLibrary.Abs` (`self.Speed`)) 10.0)
    (`self.K2_AddActorLocalRotation` (`KismetMathLibrary.MakeRotator` 0.0 0.0 (* (* (`GameplayStatics.GetWorldDeltaSeconds`) -60.0) (/ (`self.Speed`) (`self.SpeedMAx`)))))))

(fn `DriveNeutral`
  (bind _output_get (set `self.Speed` (`KismetMathLibrary.FInterpTo` (`self.Speed`) 0.0 (`GameplayStatics.GetWorldDeltaSeconds`) 3.0)))
  (`self.K2_AddActorLocalOffset` (`KismetMathLibrary.MakeVector` (* _output_get (`GameplayStatics.GetWorldDeltaSeconds`)))))

(fn `DriveRight`
  (if (> (`KismetMathLibrary.Abs` (`self.Speed`)) 10.0)
    (`self.K2_AddActorLocalRotation` (`KismetMathLibrary.MakeRotator` 0.0 0.0 (* (* (`GameplayStatics.GetWorldDeltaSeconds`) 60.0) (/ (`self.Speed`) (`self.SpeedMAx`)))))))

(fn `DriveUp`
  (bind _output_get (set `self.Speed` (`KismetMathLibrary.FClamp` (+ (`self.Speed`) (* 500.0 (`GameplayStatics.GetWorldDeltaSeconds`))) 0.0 (`self.SpeedMAx`))))
  (`self.K2_AddActorLocalOffset` (`KismetMathLibrary.MakeVector` (* _output_get (`GameplayStatics.GetWorldDeltaSeconds`)))))

(fn `UserConstructionScript`)